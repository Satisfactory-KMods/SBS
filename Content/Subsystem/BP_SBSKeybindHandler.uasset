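; Satisfactory mod subsystem that adds SBS to the build menu and handles its blueprint keybind.
; A pre-widget hook on the build menu checks that Schematic 4-5 is purchased, appends a tab if its label is absent, then injects the SBS main widget beside the browser.
; The SBS.OpenBlueprint input pops all open widgets and opens the blueprint widget through the HUD, unless it is already showing.
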(event `self.ReceiveBeginPlay`
  (`parent.ReceiveBeginPlay`)
  (`self.EnableInput` (`KBFL_Player.GetFGController`))
  (`KBFL_Widgets.BindOnPreWidget` "/Game/FactoryGame/Interface/UI/InGame/BuildMenu/Prototype/Widget_BuildMenu.Widget_BuildMenu_C" (delegate `OnPlayerInventoryOpen`)))

(event `OnPlayerInventoryOpen`
  (params (Widget :type "UserWidget Object Reference"))
  (if (`FGSchematicManager.IsSchematicPurchased` (`FGSchematicManager.Get` null) "/Game/FactoryGame/Schematics/Progression/Schematic_4-5.Schematic_4-5_C")
    (bind _aswidget_build_menu (cast `/Game/FactoryGame/Interface/UI/InGame/BuildMenu/Prototype/Widget_BuildMenu` Widget))
    (bind _widget_window_darkmode (`/Game/FactoryGame/Interface/UI/InGame/BuildMenu/Prototype/Widget_BuildMenu.Widget_Window_DarkMode` _aswidget_build_menu))
    (bind (_outtabs _hasadded) (`self.Append` (`/Game/FactoryGame/Interface/UI/Widget_Window_DarkMode.mTabs` _widget_window_darkmode)))
    (set `/Game/FactoryGame/Interface/UI/Widget_Window_DarkMode.mTabs` _outtabs _widget_window_darkmode)
    (if _hasadded
      (bind _returnvalue (`|CreateWidget` "/SBS/Widget/Widget_SBS_Main.Widget_SBS_Main_C" null (`/Game/FactoryGame/Interface/UI/InGame/BuildMenu/Prototype/Widget_BuildMenu.BPW_BlueprintMenu` _aswidget_build_menu) _widget_window_darkmode))
      (bind _ashorizontal_box (cast `HorizontalBox` (`Widget.GetParent` (`/Game/FactoryGame/Interface/UI/InGame/BuildMenu/Prototype/Widget_BuildMenu.mBrowser_Builder` _aswidget_build_menu))))
      (`HorizontalBox.AddChildToHorizontalBox` _ashorizontal_box _returnvalue))
    (else
      (`BlueprintLoggingLibrary.LogDisplay` "Unlock Schematic 4-5 for SBS!"))))

(event `InputAction|SBS.OpenBlueprint`
  (params (Key :type "Key Structure"))
  (bind _returnvalue (`KBFL_Player.GetFGController`))
  (bind _mblueprintwidget (`self.mBlueprintWidget`))
  (bind _gameui (`/Game/FactoryGame/Interface/UI/HUDHelpers/HUDHelpers.GetFGGameUI` _returnvalue))
  (:`Pressed`
    (`/Engine/EditorBlueprintResources/StandardMacros.IsValid` _returnvalue
      (:`Is Valid`
        (bind _outhud (`/Game/FactoryGame/Interface/UI/HUDHelpers/BPFL_HudHelperBadRef.GetBPHUD` _returnvalue))
        (`/Engine/EditorBlueprintResources/StandardMacros.IsValid` _outhud
          (:`Is Valid`
            (if (`KismetSystemLibrary.IsValidClass` _mblueprintwidget)
              (`/Engine/EditorBlueprintResources/StandardMacros.IsValid` (`FGGameUI.GetInteractWidgetOfClass` _gameui _mblueprintwidget)
                (:`Is Not Valid`
                  (`FGGameUI.PopAllWidgets` _gameui)
                  (`FGHUD.OpenInteractUI` _outhud _mblueprintwidget self))))))))))

(fn `Append`
  (params (Tabs :type "Array of /Game/FactoryGame/Interface/UI/InGame/-Shared/ImageAndText Structure (by ref)"))
  (returns (OutTabs :type "Array of /Game/FactoryGame/Interface/UI/InGame/-Shared/ImageAndText Structure") (HasAdded :type Boolean))
  (locals (contains :type Boolean))
  (bind (_mtab_texture _mtab_text) (break `/Game/FactoryGame/Interface/UI/InGame/-Shared/ImageAndText` (`self.mTab`)))
  (set `local.contains` false)
  (for _array_element Tabs
    (if (`KismetTextLibrary.EqualEqual_TextText` _mtab_text (`.Text_5_FD671CE446AF05CA543E228C049AB0F9` (break `/Game/FactoryGame/Interface/UI/InGame/-Shared/ImageAndText` _array_element)))
      (return Tabs false)))
  (`KismetArrayLibrary.Array_Add` Tabs (`self.mTab`))
  (return Tabs true))

(fn `OpenWidget`
  (params (WidgetClass :type "FGInteractWidget Class Reference"))
  (bind _returnvalue (`KBFL_Player.GetFGController`))
  (`/Engine/EditorBlueprintResources/StandardMacros.IsValid` _returnvalue
    (:`Is Valid`
      (bind _outhud (`/Game/FactoryGame/Interface/UI/HUDHelpers/BPFL_HudHelperBadRef.GetBPHUD` _returnvalue))
      (`/Engine/EditorBlueprintResources/StandardMacros.IsValid` _outhud
        (:`Is Valid`
          (if (`KismetSystemLibrary.IsValidClass` WidgetClass)
            (`FGHUD.OpenInteractUI` _outhud WidgetClass self)))))))

(fn `UserConstructionScript`)